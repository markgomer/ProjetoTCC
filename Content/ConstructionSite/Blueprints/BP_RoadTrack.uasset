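; BP_RoadTrack is a construction-script actor that builds a road track from spline mesh components along its spline.
; SplineMeshVar selects the layout: one segment between each pair of spline points, or segments at fixed Spacing along the spline's length.
; Point mode uses the spline's own tangents, while spacing mode uses direction times TangentScale.
; Both modes share the scaling step, which applies MeshSize to both ends of each segment.
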(fn `UserConstructionScript`
  (bind _conponent_1 (`self.Conponent 1`))
  (bind _spline (`self.Spline`))
  (bind _spline_2 (`self.Spline`))
  (bind _mesh_size (`self.Mesh Size`))
  (bind _points (`self.Points`))
  (bind _spacing (`self.Spacing`))
  (bind _tangent_scale (`self.Tangent Scale`))
  (bind (_location _tangent) (`SplineComponent.GetLocationAndTangentAtSplinePoint` _spline _points "Local"))
  (bind (_location_2 _tangent_2) (`SplineComponent.GetLocationAndTangentAtSplinePoint` _spline (+ _points 1) "Local"))
  (set `self.Conponent 1` null)
  (switch `int` (`self.Spline Mesh Var`)
    (:`0`
      (for _index (range (+ (- (`SplineComponent.GetNumberOfSplinePoints` (`self.Spline`)) 2) 1))
        (set `self.Points` _index)
        (bind _returnvalue (`AddComponent|NODE_AddSplineMeshComponent-13`))
        (set `self.Conponent 1` _returnvalue)
        (`SplineMeshComponent.SetStartAndEnd` _conponent_1 _location _tangent _location_2 _tangent_2 true)
        (`SplineMeshComponent.SetStartScale` _conponent_1 (`KismetMathLibrary.MakeVector2D` _mesh_size _mesh_size) true :!label _label)
        (`SplineMeshComponent.SetEndScale` _conponent_1 (`KismetMathLibrary.MakeVector2D` _mesh_size _mesh_size) true)))
    (:`1`
      (for _index_2 (range (+ (`.ReturnValue` (`KismetMathLibrary.FMod` (`SplineComponent.GetSplineLength` _spline_2) _spacing)) 1))
        (bind _returnvalue_2 (`AddComponent|NODE_AddSplineMeshComponent-14`))
        (set `self.Conponent 1` _returnvalue_2)
        (bind _returnvalue_3 (* _index_2 _spacing))
        (bind _returnvalue_4 (+ _returnvalue_3 _spacing))
        (`SplineMeshComponent.SetStartAndEnd` _conponent_1 (`SplineComponent.GetLocationAtDistanceAlongSpline` _spline_2 _returnvalue_3 "Local") (* (`SplineComponent.GetDirectionAtDistanceAlongSpline` _spline_2 _returnvalue_3 "Local") _tangent_scale) (`SplineComponent.GetLocationAtDistanceAlongSpline` _spline_2 _returnvalue_4 "Local") (* (`SplineComponent.GetDirectionAtDistanceAlongSpline` _spline_2 _returnvalue_4 "Local") _tangent_scale) true)
        (goto _label)))))