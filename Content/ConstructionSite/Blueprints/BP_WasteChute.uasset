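; BP_WasteChute is a construction-site waste chute that builds itself along a spline in the construction script.
; The Wire graph places one spline mesh every Spacing units along the spline, with each segment's end offset by Shift and its tangents scaled by TangentScale.
; Each segment gets its own dynamic instance of MI_WasteChute01, with diffuse color set from the Color variable.
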(fn `UserConstructionScript`
  (bind _spline (`self.Spline`))
  (bind _spacing (`self.Spacing`))
  (bind _tangent_scale (`self.Tangent Scale`))
  (for _index (range (+ (`.ReturnValue` (`KismetMathLibrary.FMod` (`SplineComponent.GetSplineLength` _spline) _spacing)) 1))
    (bind _returnvalue (`AddComponent|NODE_AddSplineMeshComponent-4`))
    (bind _returnvalue_2 (* _index _spacing))
    (bind _returnvalue_3 (+ _returnvalue_2 (- _spacing (`self.Shift`))))
    (`SplineMeshComponent.SetStartAndEnd` _returnvalue (`SplineComponent.GetLocationAtDistanceAlongSpline` _spline _returnvalue_2 "Local") (* (`SplineComponent.GetDirectionAtDistanceAlongSpline` _spline _returnvalue_2 "Local") _tangent_scale) (`SplineComponent.GetLocationAtDistanceAlongSpline` _spline _returnvalue_3 "Local") (* (`SplineComponent.GetDirectionAtDistanceAlongSpline` _spline _returnvalue_3 "Local") _tangent_scale) true)
    (bind _returnvalue_4 (`KismetMaterialLibrary.CreateDynamicMaterialInstance` "/Game/ConstructionSite/Materials/ConstructionSite/MI_WasteChute01.MI_WasteChute01"))
    (`PrimitiveComponent.SetMaterial` _returnvalue 0 _returnvalue_4)
    (`MaterialInstanceDynamic.SetVectorParameterValue` _returnvalue_4 "diffuse color" (`self.Color`))))