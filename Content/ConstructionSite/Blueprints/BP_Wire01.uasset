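; Construction-site wire Blueprint that builds spline meshes along a Spline in the construction script.
; SplineMeshVar selects one segment between each pair of spline points, or segments at Spacing intervals with TangentScale-scaled tangents.
; WireVar selects the mesh component variant and whether a second material slot is set, and WireSize scales the cross-section.
; Dynamic instances of MI_Gray receive color, dirt and surface parameters, plus a texture set chosen by TextureVar.
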(fn `UserConstructionScript`
  (bind _conponent_1 (`self.Conponent 1`))
  (bind _spline (`self.Spline`))
  (bind _spline_2 (`self.Spline`))
  (bind _wire_size (`self.Wire Size`))
  (bind _points (`self.Points`))
  (bind _spacing (`self.Spacing`))
  (bind _tangent_scale (`self.Tangent Scale`))
  (bind _color2 (`self.Color2`))
  (bind (_location _tangent) (`SplineComponent.GetLocationAndTangentAtSplinePoint` _spline _points "Local"))
  (bind (_location_2 _tangent_2) (`SplineComponent.GetLocationAndTangentAtSplinePoint` _spline (+ _points 1) "Local"))
  (set `self.Conponent 1` null)
  (switch `int` (`self.Spline Mesh Var`)
    (:`Default`
      (for _index (range (+ (- (`SplineComponent.GetNumberOfSplinePoints` (`self.Spline`)) 2) 1)) :!label _label
        (set `self.Points` _index)
        (switch `int` (`self.Wire Var`)
          (:`Default`
            (bind _returnvalue (`AddComponent|NODE_AddSplineMeshComponent-13` :!label _label_2))
            (set `self.Conponent 1` _returnvalue))
          (:`0`
            (goto _label_2))
          (:`1`
            (bind _returnvalue_2 (`AddComponent|NODE_AddSplineMeshComponent-1`))
            (set `self.Conponent 1` _returnvalue_2))
          (:`2`
            (bind _returnvalue_3 (`AddComponent|NODE_AddSplineMeshComponent-2`))
            (set `self.Conponent 1` _returnvalue_3)))
        (`SplineMeshComponent.SetStartAndEnd` _conponent_1 _location _tangent _location_2 _tangent_2 true)
        (`SplineMeshComponent.SetStartScale` _conponent_1 (`KismetMathLibrary.MakeVector2D` _wire_size _wire_size) true :!label _label_3)
        (`SplineMeshComponent.SetEndScale` _conponent_1 (`KismetMathLibrary.MakeVector2D` _wire_size _wire_size) true)
        (switch `int` (`self.Wire Var`)
          (:`Default`
            _)
          (:`0`
            _)
          (:`1`
            _)
          (:`2`
            _)
          (:`3`
            (bind _returnvalue_4 (`KismetMaterialLibrary.CreateDynamicMaterialInstance` "/Game/ConstructionSite/Materials/MI_Gray.MI_Gray" :!label _label_4))
            (`PrimitiveComponent.SetMaterial` _conponent_1 1 _returnvalue_4))
          (:`4`
            (goto _label_4))
          (:`5`
            (goto _label_4)))
        (bind _returnvalue_5 (`KismetMaterialLibrary.CreateDynamicMaterialInstance` "/Game/ConstructionSite/Materials/MI_Gray.MI_Gray"))
        (`PrimitiveComponent.SetMaterial` _conponent_1 0 _returnvalue_5)
        (`MaterialInstanceDynamic.SetVectorParameterValue` _returnvalue_5 "diffuse color" (`self.Color`))
        (`MaterialInstanceDynamic.SetVectorParameterValue` _returnvalue_4 "diffuse color" (`self.Color`))
        (`MaterialInstanceDynamic.SetScalarParameterValue` _returnvalue_5 "spec" (`self.Specular`))
        (`MaterialInstanceDynamic.SetScalarParameterValue` _returnvalue_4 "spec" (`self.Specular`))
        (`MaterialInstanceDynamic.SetScalarParameterValue` _returnvalue_5 "Roughness" (`self.Roughness`))
        (`MaterialInstanceDynamic.SetScalarParameterValue` _returnvalue_4 "Roughness" (`self.Roughness`))
        (`MaterialInstanceDynamic.SetScalarParameterValue` _returnvalue_5 "Metallic" (`self.Metallic`))
        (`MaterialInstanceDynamic.SetScalarParameterValue` _returnvalue_4 "Metallic" (`self.Metallic`))
        (`MaterialInstanceDynamic.SetVectorParameterValue` _returnvalue_5 "dirt color" (`self.Dirt Color`))
        (`MaterialInstanceDynamic.SetVectorParameterValue` _returnvalue_4 "dirt color" (`self.Dirt Color`))
        (`MaterialInstanceDynamic.SetVectorParameterValue` _returnvalue_5 "additional diffuse color" _color2)
        (`MaterialInstanceDynamic.SetVectorParameterValue` _returnvalue_4 "diffuse color" _color2)
        (switch `int` (`self.Texture var`)
          (:`Default`
            (`MaterialInstanceDynamic.SetTextureParameterValue` _returnvalue_5 "Diffuse" "/Game/ConstructionSite/Textures/BaseTextures/T_BW_D.T_BW_D" :!label _label_5)
            (`MaterialInstanceDynamic.SetTextureParameterValue` _returnvalue_4 "Diffuse" "/Game/ConstructionSite/Textures/BaseTextures/T_BW_D.T_BW_D")
            (`MaterialInstanceDynamic.SetTextureParameterValue` _returnvalue_5 "Normal" "/Game/ConstructionSite/Textures/BaseTextures/T_B_N.T_B_N")
            (`MaterialInstanceDynamic.SetTextureParameterValue` _returnvalue_4 "Normal" "/Game/ConstructionSite/Textures/BaseTextures/T_B_N.T_B_N")
            (`MaterialInstanceDynamic.SetTextureParameterValue` _returnvalue_5 "SRMH" "/Game/ConstructionSite/Textures/BaseTextures/T_BG_D.T_BG_D")
            (`MaterialInstanceDynamic.SetTextureParameterValue` _returnvalue_4 "SRMH" "/Game/ConstructionSite/Textures/BaseTextures/T_BG_D.T_BG_D"))
          (:`0`
            (goto _label_5))
          (:`1`
            (`MaterialInstanceDynamic.SetTextureParameterValue` _returnvalue_5 "Diffuse" "/Game/ConstructionSite/Textures/Blueprint/T_Wire01_D.T_Wire01_D")
            (`MaterialInstanceDynamic.SetTextureParameterValue` _returnvalue_5 "Normal" "/Game/ConstructionSite/Textures/Blueprint/T_Wire01_N.T_Wire01_N")
            (`MaterialInstanceDynamic.SetTextureParameterValue` _returnvalue_5 "SRMH" "/Game/ConstructionSite/Textures/Blueprint/T_Wire01_SRM.T_Wire01_SRM"))
          (:`2`
            (`MaterialInstanceDynamic.SetTextureParameterValue` _returnvalue_5 "Diffuse" "/Game/ConstructionSite/Textures/Blueprint/T_Wire02_D.T_Wire02_D")
            (`MaterialInstanceDynamic.SetTextureParameterValue` _returnvalue_5 "Normal" "/Game/ConstructionSite/Textures/BaseTextures/T_B_N.T_B_N")
            (`MaterialInstanceDynamic.SetTextureParameterValue` _returnvalue_5 "SRMH" "/Game/ConstructionSite/Textures/BaseTextures/T_BG_D.T_BG_D")))))
    (:`0`
      (goto _label))
    (:`1`
      (for _index_2 (range (+ (`.ReturnValue` (`KismetMathLibrary.FMod` (`SplineComponent.GetSplineLength` _spline_2) _spacing)) 1))
        (switch `int` (`self.Wire Var`)
          (:`Default`
            (bind _returnvalue_6 (`AddComponent|NODE_AddSplineMeshComponent-4` :!label _label_6))
            (set `self.Conponent 1` _returnvalue_6))
          (:`0`
            (goto _label_6))
          (:`1`
            (bind _returnvalue_7 (`AddComponent|NODE_AddSplineMeshComponent-5`))
            (set `self.Conponent 1` _returnvalue_7))
          (:`2`
            (bind _returnvalue_8 (`AddComponent|NODE_AddSplineMeshComponent-6`))
            (set `self.Conponent 1` _returnvalue_8)))
        (bind _returnvalue_9 (* _index_2 _spacing))
        (bind _returnvalue_10 (+ _returnvalue_9 _spacing))
        (`SplineMeshComponent.SetStartAndEnd` _conponent_1 (`SplineComponent.GetLocationAtDistanceAlongSpline` _spline_2 _returnvalue_9 "Local") (* (`SplineComponent.GetDirectionAtDistanceAlongSpline` _spline_2 _returnvalue_9 "Local") _tangent_scale) (`SplineComponent.GetLocationAtDistanceAlongSpline` _spline_2 _returnvalue_10 "Local") (* (`SplineComponent.GetDirectionAtDistanceAlongSpline` _spline_2 _returnvalue_10 "Local") _tangent_scale) true)
        (goto _label_3)))))